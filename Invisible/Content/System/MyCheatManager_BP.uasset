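; Debug cheat manager with commands to toggle enemy silhouette visibility and search-edge debug drawing.
; VisibleEnemy ORs a visibility mask into the custom depth stencil of every BP_Enemy silhouette mesh and prints the result.
; InvisibleEnemy ORs in the inverted mask instead of ANDing it, so the visibility bits are not cleared.
; VisibleSearch and InvisibleSearch switch DebugDraw on every BP_SearchEgde actor and print each state.
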(event `self.VisibleEnemy`
  (bind _outactors (`GameplayStatics.GetAllActorsOfClass` "/Game/Enemy/BP_Enemy.BP_Enemy_C"))
  (for _array_element _outactors
    (bind _silhouetteskeltal (`Enemy.silhouetteSkeltal` _array_element))
    (bind _returnvalue (`KismetMathLibrary.Or_IntInt` (`PrimitiveComponent.CustomDepthStencilValue` _silhouetteskeltal) (`self.EnemyVisibleMaskValue`)))
    (`PrimitiveComponent.SetCustomDepthStencilValue` _silhouetteskeltal _returnvalue)
    (`KismetSystemLibrary.PrintString` (`KismetStringLibrary.Conv_IntToString` _returnvalue))))

(event `self.InvisibleEnemy`
  (bind _outactors (`GameplayStatics.GetAllActorsOfClass` "/Game/Enemy/BP_Enemy.BP_Enemy_C"))
  (for _array_element _outactors
    (bind _silhouetteskeltal (`Enemy.silhouetteSkeltal` _array_element))
    (`PrimitiveComponent.SetCustomDepthStencilValue` _silhouetteskeltal (`KismetMathLibrary.Or_IntInt` (`PrimitiveComponent.CustomDepthStencilValue` _silhouetteskeltal) (`KismetMathLibrary.Not_Int` (`self.EnemyVisibleMaskValue`))))))

(event `self.VisibleSearch`
  ;[1 1 1] DebugSearch
  (bind _outactors (`GameplayStatics.GetAllActorsOfClass` "/Game/Enemy/BP_SearchEgde.BP_SearchEgde_C"))
  (for _array_element _outactors
    (set `SearchEgde.debugDraw` 1 _array_element)
    (`KismetSystemLibrary.PrintString` (`KismetStringLibrary.Concat_StrStr` (`KismetSystemLibrary.GetObjectName` _array_element) (`KismetStringLibrary.Concat_StrStr` ": " (`KismetStringLibrary.Conv_IntToString` (`SearchEgde.debugDraw` _array_element)))))))

(event `self.InvisibleSearch`
  ;[1 1 1] DebugSearch
  (bind _outactors (`GameplayStatics.GetAllActorsOfClass` "/Game/Enemy/BP_SearchEgde.BP_SearchEgde_C"))
  (for _array_element _outactors
    (set `SearchEgde.debugDraw` 0 _array_element)
    (`KismetSystemLibrary.PrintString` (`KismetStringLibrary.Concat_StrStr` (`KismetSystemLibrary.GetObjectName` _array_element) (`KismetStringLibrary.Concat_StrStr` ": " (`KismetStringLibrary.Conv_IntToString` (`SearchEgde.debugDraw` _array_element)))))))