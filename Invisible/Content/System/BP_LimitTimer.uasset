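; Countdown timer actor that shows remaining time in a UI_RemainTime widget and drives the last-minute alarm.
; Tick updates the widget and, at 60 seconds, plays a one-off alert and turns all cached spotlight actors to red material and a tinted light, blinking until the final ten seconds hold it steady.
; HUD helpers spawn starting-time text, retrying by timer if the HUD cast fails, and once-only minute notices.
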(event `self.ReceiveBeginPlay`
  (set `self.play_sound` false)
  (bind _outactors (`GameplayStatics.GetAllActorsOfClass` "/Game/module/Light/BP_SpotLight.BP_SpotLight_C"))
  (set `self.spot_light_array` _outactors)
  (bind _outactors_2 (`GameplayStatics.GetAllActorsOfClass` "/Game/module/Light/BP_SpotLight_Flash.BP_SpotLight_Flash_C"))
  (set `self.spot_light_frash_array` _outactors_2)
  (bind _returnvalue (`|CreateWidget` "/Game/UI/UI_RemainTime.UI_RemainTime_C" (`GameplayStatics.GetPlayerController` 0)))
  (`UserWidget.AddToViewport` _returnvalue 0)
  (set `self.RemainTime` _returnvalue))

(event `self.ReceiveTick`
  (params (DeltaSeconds :type "Float (single-precision)"))
  (bind _returnvalue (`self.GetLimitTimer`))
  (bind _returnvalue_2 (`self.GetLimitTimer`))
  (bind _returnvalue_3 (* (`self.ChangeLightColor`) (`KismetMathLibrary.SelectFloat` 1.0 (`KismetMathLibrary.SelectFloat` 1.0 0.0 (<= (`KismetMathLibrary.Fraction` _returnvalue) 0.7)) (<= _returnvalue 10.0))))
  (`/Game/UI/UI_RemainTime.Set Time` (`self.RemainTime`) _returnvalue_2)
  (if (<= _returnvalue_2 60.0)
    (if (not (`self.play_sound`))
      (set `self.play_sound` true)
      (`/Game/System/SoundUtil.PlaySound` "Alert" (`self.K2_GetActorLocation` (`ActorComponent.GetOwner` (`Character.CapsuleComponent` (`GameplayStatics.GetPlayerCharacter` 0))))))
    (for _array_element (`self.spot_light_array`)
      (`LightComponent.SetLightColor` (`/Game/module/Light/BP_SpotLight.SpotLight` _array_element) _returnvalue_3 true)
      (`PrimitiveComponent.SetMaterial` (`/Game/module/Light/BP_SpotLight.LightBody` _array_element) 0 "/Game/module/Light/RedLightMaterial.RedLightMaterial"))
    (for _array_element_2 (`self.spot_light_frash_array`)
      (`LightComponent.SetLightColor` (`/Game/module/Light/BP_SpotLight_Flash.SpotLight` _array_element_2) _returnvalue_3 true)
      (`PrimitiveComponent.SetMaterial` (`/Game/module/Light/BP_SpotLight_Flash.LightBody` _array_element_2) 0 "/Game/module/Light/RedLightMaterial.RedLightMaterial"))))

(event `self.InitializeHUDText`
  (`self.InitializeHUDText_Impl`))

(fn `InitializeHUDText_Impl`
  (bind _returnvalue (`self.GetLimitTimer`))
  (bind _hud (`self.GetPlayerHUD`)
    (:`Succeed`
      (`KismetSystemLibrary.PrintString` (`KismetStringLibrary.Conv_DoubleToString` _returnvalue))
      (switch `int` (`KismetMathLibrary.FFloor` (/ (+ _returnvalue 1.0) 60.0))
        (:`Default`
          (`PlayerHUD.SpawnTextUI` _hud "START_5M"))
        (:`3`
          (`PlayerHUD.SpawnTextUI` _hud "START_3M"))
        (:`4`
          (`PlayerHUD.SpawnTextUI` _hud "START_4M"))))
    (:`Failed`
      (`KismetSystemLibrary.K2_SetTimerDelegate` (`|CreateDelegate` :!event `InitializeHUDText_Impl`)))))

(fn `SpawnLimit60TextOnce`
  (params (RemainTimeMinite :type Integer))
  (bind _hud (`self.GetPlayerHUD`)
    (:`Succeed`
      (switch `int` RemainTimeMinite
        (:`1`
          ;[1 1 1] それぞれ一回だけ呼ぶようにする
          (`/Engine/EditorBlueprintResources/StandardMacros.DoOnce` false
            (:`Completed`
              (`PlayerHUD.SpawnTextUI` _hud "LIMIT_60"))))
        (:`2`
          (`/Engine/EditorBlueprintResources/StandardMacros.DoOnce` false
            (:`Completed`
              (`PlayerHUD.SpawnTextUI` _hud "LIMIT_120"))))
        (:`3`
          (`/Engine/EditorBlueprintResources/StandardMacros.DoOnce` false
            (:`Completed`
              (`self.EqualStartTime` RemainTimeMinite
                (:`NotEqual`
                  (`PlayerHUD.SpawnTextUI` _hud "LIMIT_180"))))))
        (:`4`
          (`/Engine/EditorBlueprintResources/StandardMacros.DoOnce` false
            (:`Completed`
              (`self.EqualStartTime` RemainTimeMinite
                (:`NotEqual`
                  (`PlayerHUD.SpawnTextUI` _hud "LIMIT_240"))))))))))

(fn `UserConstructionScript`)