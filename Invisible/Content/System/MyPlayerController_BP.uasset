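; MyPlayerController_BP is a player controller Blueprint that handles input for quitting the game.
; The Exit input action quits the game immediately.
; StartButton and BackButton each track their held state in a flag, and pressing either one while the other is held triggers the same quit, forming a two-button chord.
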(event `self.ReceiveTick`
  (params (DeltaSeconds :type "Float (single-precision)")))

(event `InputAction|Exit`
  (params (Key :type "Key Structure"))
  (:`Pressed`
    (`KismetSystemLibrary.QuitGame` null "Quit" :!label _label)))

(event `InputAction|StartButton`
  (params (Key :type "Key Structure"))
  (:`Pressed`
    (set `self.bIsPressedStart` true)
    (if (and (`self.bIsPressedStart`) (`self.bIsPressedBack`)) :!label _label_2
      (goto _label)))
  (:`Released`
    (set `self.bIsPressedStart` false)))

(event `InputAction|BackButton`
  (params (Key :type "Key Structure"))
  (:`Pressed`
    (set `self.bIsPressedBack` true)
    (goto _label_2))
  (:`Released`
    (set `self.bIsPressedBack` false)))

(fn `UserConstructionScript`)