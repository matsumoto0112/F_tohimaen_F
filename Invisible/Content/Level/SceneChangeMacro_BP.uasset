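; Blueprint macro that changes scenes by fading out before opening the named level.
; SceneChange starts a non-blocking, hidden stream load of the next level, then adds a SceneFade_UI widget and starts its timed fade-out.
; A looping timer, set to the frame delta, polls the widget until the fade ends, then clears itself with a negative time, destroys sound objects and opens the level by name.
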(event Custom|Wait
  (bind _isend (Default|IsFadeEnd (stale _returnvalue)))
  (if _isend
    (Utilities|Time|SetTimerbyEvent (delegate Custom|Wait) -1.0)
    (CallFunction|DestroySoundObjects)
    (Game|OpenLevel(byName) (stale _nextlevelname))
    (return)))