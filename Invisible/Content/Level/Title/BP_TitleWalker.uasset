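; BP_TitleWalker is a title-level actor that circles endlessly while playing positional footstep sounds.
; Each tick advances an angle by Speed, independent of delta time, and places the actor on a small horizontal circle around the world origin.
; A delta-time timer triggers the title footstep sound at the actor's location, subtracting Interval each time so leftover time carries over.
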(event `self.ReceiveTick`
  (params (DeltaSeconds :type "Float (single-precision)"))
  (`self.TimeUpdate` DeltaSeconds)
  (`self.CircleWalk`)
  (bind _istiming (`self.IsPlayWalkSoundTiming`))
  (if _istiming
    (`self.DecreaseTime`)
    (`self.PlayWalkSound`)))

(fn `CircleWalk`
  (bind _angle (`self.Angle`))
  (set `self.Angle` (+ (`self.Angle`) (`self.Speed`)))
  (`self.K2_SetActorLocation` (* (`KismetMathLibrary.MakeVector` (`KismetMathLibrary.DegSin` _angle) (`KismetMathLibrary.DegCos` _angle)) 50.0)))

(fn `DecreaseTime`
  (set `self.Timer` (- (`self.Timer`) (`self.Interval`))))

(fn `IsPlayWalkSoundTiming`
  (returns (IsTiming :type Boolean))
  (return (>= (`self.Timer`) (`self.Interval`))))

(fn `PlayWalkSound`
  (`/Game/System/SoundUtil.PlaySound` "Title_FootSteps" (`self.K2_GetActorLocation`) self))

(fn `TimeUpdate`
  (params (DeltaSeconds :type "Float (double-precision)"))
  (set `self.Timer` (+ (`self.Timer`) DeltaSeconds)))

(fn `UserConstructionScript`)