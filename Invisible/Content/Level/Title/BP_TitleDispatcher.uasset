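; Title-level dispatcher that starts the title scene, owns its UI and handles moves to other scenes.
; On BeginPlay it sets up sound objects and volume, shows the title widget and prepares the config widget with settings from MyGameInstance.
; Both widgets receive a reference back to this dispatcher.
; ConfigMode and ReturnPrev swap the two screens and track the active UI, while SceneChange switches levels with a fade.
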(event `self.ReceiveBeginPlay`
  (`/Game/Level/SceneChangeFunction_BP.CreateSoundObjects` 30)
  (`/Game/Level/F_SceneStart.SceneStart` 0.2)
  (bind _returnvalue (`|CreateWidget` "/Game/Level/Title/Title_UI_BP.Title_UI_BP_C" (`GameplayStatics.GetPlayerController` 0)))
  (bind _output_get (set `self.TitleUI` _returnvalue))
  (set `/Game/Level/Title/Title_UI_BP.Dispatcher` self _output_get)
  (`UserWidget.AddToViewport` _output_get 0)
  (bind _returnvalue_2 (`|CreateWidget` "/Game/Level/Config/BP_Config_UI.BP_Config_UI_C" (`GameplayStatics.GetPlayerController` 0)))
  (set `self.ConfigUI` _returnvalue_2)
  (bind _asmy_game_instance (cast `MyGameInstance` (`GameplayStatics.GetGameInstance`)))
  (`/Game/Level/Config/BP_Config_UI.Init` (`self.ConfigUI`) (`MyGameInstance.GetConfigParams` _asmy_game_instance) self)
  (set `self.UI` (`self.TitleUI`))
  (`/Game/System/BP_SetSoundClassVolume.SetSoundClassVolume`))

(event `self.ReceiveTick`
  (params (DeltaSeconds :type "Float (single-precision)")))

(event `SceneChange`
  (params (NextSceneName :type Name))
  (`/Game/Level/SceneChangeMacro_BP.SceneChange` NextSceneName 1.0))

(event `/Game/Level/Config/BP_ConfigDispather.ReturnPrev`
  (bind _titleui (`self.TitleUI`))
  (`Widget.RemoveFromParent` (`self.ConfigUI`))
  (`UserWidget.AddToViewport` _titleui 0)
  (set `self.UI` _titleui))

(fn `ConfigMode`
  (bind _configui (`self.ConfigUI`))
  (`Widget.RemoveFromParent` (`self.TitleUI`))
  (`UserWidget.AddToViewport` _configui 0)
  (set `self.UI` _configui))

(fn `UserConstructionScript`)