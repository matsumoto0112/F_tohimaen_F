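; SimpleLevelController_BP is a level controller for a simple scene that advances to the next level when the player confirms.
; On BeginPlay it creates the sound objects and starts the scene.
; Releasing the SystemDecision input passes a DoOnce, plays the decision sound at the world origin through MyGameInstance's sound system, and after a short delay calls SceneChange to fade to NextLevelName.
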(event `self.ReceiveBeginPlay`
  (`/Game/Level/SceneChangeFunction_BP.CreateSoundObjects` (`self.MaxSoundObjectNum`))
  (`/Game/Level/F_SceneStart.SceneStart` 0.2))

(event `InputAction|SystemDecision`
  (params (Key :type "Key Structure"))
  (:`Released`
    (`/Engine/EditorBlueprintResources/StandardMacros.DoOnce` false
      (:`Completed`
        (bind _asmy_game_instance (cast `MyGameInstance` (`GameplayStatics.GetGameInstance`)))
        (`SoundSystem.play3DSound` (`MyGameInstance.getSoundSystem` _asmy_game_instance) "System_Decision" (`KismetMathLibrary.MakeVector` 0.0) null)
        (`KismetSystemLibrary.Delay` 0.5)
        (`/Game/Level/SceneChangeMacro_BP.SceneChange` (`self.NextLevelName`) 1.0)))))

(fn `UserConstructionScript`)