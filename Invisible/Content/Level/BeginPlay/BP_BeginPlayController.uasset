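; BP_BeginPlayController runs a movie screen that leads into the Title level.
; On BeginPlay it creates sound objects, adds the BP_MovieUI widget to the viewport, opens the media source and binds to its end-reached event.
; The movie ending or a SystemDecision press, which also plays a confirm sound, starts a faded scene change to Title.
; A SceneChaning flag lets only the first trigger start the transition.
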(event `self.ReceiveBeginPlay`
  (bind _media (`self.Media`))
  (`/Game/Level/SceneChangeFunction_BP.CreateSoundObjects` 3)
  (bind _returnvalue (`|CreateWidget` "/Game/Level/BeginPlay/BP_MovieUI.BP_MovieUI_C"))
  (`UserWidget.AddToViewport` _returnvalue 0)
  (`MediaPlayer.OpenSource` _media "/Game/Movies/body.body")
  (add `MediaPlayer.OnEndReached` _media (delegate `OnEndReached_イベント_0`)))

(event `OnEndReached_イベント_0`
  (if (not (`self.bSceneChaning`))
    (set `self.bSceneChaning` true)
    (`/Game/Level/SceneChangeMacro_BP.SceneChange` "Title" 2.0 :!label _label)))

(event `InputAction|SystemDecision`
  (params (Key :type "Key Structure"))
  (:`Pressed`
    (if (not (`self.bSceneChaning`))
      (set `self.bSceneChaning` true)
      (`/Game/System/SoundUtil.PlaySound` "System_Decision")
      (goto _label))))

(fn `UserConstructionScript`)