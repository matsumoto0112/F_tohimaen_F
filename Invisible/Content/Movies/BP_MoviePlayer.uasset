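; Movie player actor that plays a media source with UI and sound, then fades to the next level.
; BeginPlay sets sound class volume, creates sound objects, links the media sound to the player, adds BP_MovieUI and opens the source.
; Reaching the media's end or pressing SystemDecision, which also plays a confirm sound, triggers SceneChange.
; A shared flag ensures the transition fires only once.
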(event `self.ReceiveBeginPlay`
  (bind _media (`self.Media`))
  (`/Game/System/BP_SetSoundClassVolume.SetSoundClassVolume`)
  (`MediaSoundComponent.SetMediaPlayer` (`self.MediaSound`) (`self.Media`))
  (`/Game/Level/SceneChangeFunction_BP.CreateSoundObjects` 3)
  (bind _returnvalue (`|CreateWidget` "/Game/Movies/BP_MovieUI.BP_MovieUI_C" (`GameplayStatics.GetPlayerController` 0)))
  (`UserWidget.AddToViewport` _returnvalue 0)
  (`MediaPlayer.OpenSource` _media (`self.MediaSource`))
  (add `MediaPlayer.OnEndReached` _media (delegate `OnEndReached_イベント_0`)))

(event `OnEndReached_イベント_0`
  (if (not (`self.bSceneChaning`))
    (set `self.bSceneChaning` true)
    (`/Game/Level/SceneChangeMacro_BP.SceneChange` (`self.NextSceneName`) (`self.FadeTime`) :!label _label)))

(event `InputAction|SystemDecision`
  (params (Key :type "Key Structure"))
  (:`Pressed`
    (if (not (`self.bSceneChaning`))
      (set `self.bSceneChaning` true)
      (`/Game/System/SoundUtil.PlaySound` "System_Decision")
      (goto _label))))

(fn `UserConstructionScript`)