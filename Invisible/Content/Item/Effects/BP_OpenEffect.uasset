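; BP_OpenEffect is an item effect actor that animates an "opening" material on a sphere.
; Construction creates a dynamic instance of OpenMaterial and scales the actor uniformly to MaxScale.
; BeginPlay resets the "specular" parameter to zero; while IsStart is true, Tick ramps it to one at ScaleSpeed.
; Despite that variable's name, the scale stays fixed, as the MaxScale × Specular multiply is left unconnected.
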(event `self.ReceiveBeginPlay`
  (`self.SetSpecular` 0.0))

(event `self.ReceiveTick`
  (params (DeltaSeconds :type "Float (single-precision)"))
  (`self.MaterialUpdate` DeltaSeconds))

(fn `ActorScale`
  (`self.SetActorScale3D` (* (`KismetMathLibrary.Vector_One`) (`self.MaxScale`))))

(fn `MaterialUpdate`
  (params (DeltaSeconds :type "Float (double-precision)"))
  (if (`self.IsStart`)
    (bind _output_get (set `self.specular` (`KismetMathLibrary.FClamp` (+ (* DeltaSeconds (`self.ScaleSpeed`)) (`self.specular`)))))
    (`self.SetSpecular` _output_get)
    (`self.ActorScale`)))

(fn `SetSpecular`
  (params (specular :type "Float (double-precision)"))
  (bind _output_get (set `self.specular` specular))
  (`MaterialInstanceDynamic.SetScalarParameterValue` (`self.material`) "specular" _output_get))

(fn `UserConstructionScript`
  (bind _returnvalue (`PrimitiveComponent.CreateDynamicMaterialInstance` (`self.Sphere`) 0 "/Game/Item/Effects/OpenMaterial.OpenMaterial" "None"))
  (set `self.material` _returnvalue)
  (`self.SetSpecular` (`self.specular`))
  (`self.ActorScale`))