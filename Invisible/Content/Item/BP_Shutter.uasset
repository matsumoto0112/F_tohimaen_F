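; BP_Shutter is a device-driven shutter that slides upward once opened, with no logic to close it again.
; DeviceAction sets the open flag, and DeviceActionUpdate advances a clamped timer by frame delta, derived through a GetFPS helper, instead of using its own Tick.
; The timer ratio linearly raises the actor from its BeginPlay location by Height over MovTime, without sweep.
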(event `self.ReceiveBeginPlay`
  (set `self.pos` (`self.K2_GetActorLocation`)))

(event `self.DeviceAction`
  (set `self.isOpen` true))

(event `self.DeviceActionUpdate`
  (if (`self.isOpen`)
    (if (< (`self.timer`) (`self.movTime`))
      (bind _fps (`self.GetFPS`))
      (bind _output_get (set `self.timer` (`KismetMathLibrary.FClamp` (+ (/ 1.0 _fps) (`self.timer`)) 0.0 (`self.movTime`))))
      (`self.K2_SetActorLocation` (`KismetMathLibrary.MakeVector` (.x (`self.pos`)) (.y (`self.pos`)) (+ (.z (`self.pos`)) (* (/ _output_get (`self.movTime`)) (`self.height`))))))))

(fn `GetFPS`
  (returns (fps :type "Float (double-precision)"))
  (return (/ 1.0 (`GameplayStatics.GetWorldDeltaSeconds`))))

(fn `UserConstructionScript`)