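; Sliding double-gate exit device that changes to the next level once fully open.
; DeviceAction sets the open flag, and each DeviceActionUpdate slides both doors apart along the actor's right vector, using frame-time-scaled steps clamped to OpenWidth.
; A BP_OpenEffect spawned at BeginPlay starts once the doors part, and SceneChange fires with a short fade at full width.
; An unconnected debug helper draws the open extents.
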(event `self.ReceiveBeginPlay`
  (bind _returnvalue (`|SpawnActorFromClass` "/Game/Item/Effects/BP_OpenEffect.BP_OpenEffect_C" (`self.GetTransform`) "Undefined" "OverrideRootScale" null null))
  (set `self.openEffect` _returnvalue))

(event `self.ReceiveTick`
  (params (DeltaSeconds :type "Float (single-precision)")))

(event `self.DeviceAction`
  (set `self.isOpen` true))

(event `self.DeviceActionUpdate`
  (bind _isopen (`self.open_the_door`))
  (if _isopen
    (`/Game/Level/SceneChangeMacro_BP.SceneChange` (`self.sceneChangeName`))
    (else
      (`self.EffectUpdate`))))

(fn `DebugDrawOpen`
  (bind _returnvalue (`KismetMathLibrary.MakeColor` 0.0 0.0 1.0))
  (bind _returnvalue_2 (`self.K2_GetActorRotation`))
  (bind _returnvalue_3 (* (`self.GetActorRightVector`) (`self.open_width`)))
  (bind _returnvalue_4 (`KismetMathLibrary.MakeVector` (.x (`self.K2_GetActorLocation`)) (.y (`self.K2_GetActorLocation`)) (.z (`SceneComponent.K2_GetComponentLocation` (`self.rightBox`)))))
  (bind _returnvalue_5 (+ _returnvalue_4 _returnvalue_3))
  (bind _returnvalue_6 (+ _returnvalue_4 (* _returnvalue_3 -1.0)))
  ;[1 1 1] draws
  (`KismetSystemLibrary.DrawDebugLine` _returnvalue_5 _returnvalue_6 _returnvalue 1.0 100.0)
  ;;[1 1 1] draw_right
  (`KismetSystemLibrary.DrawDebugBox` _returnvalue_5 (`BoxComponent.BoxExtent` (`self.rightBox`)) _returnvalue _returnvalue_2 1.0 100.0)
  ;;[1 1 1] draw_left
  (`KismetSystemLibrary.DrawDebugBox` _returnvalue_6 (`BoxComponent.BoxExtent` (`self.leftBox`)) _returnvalue _returnvalue_2 1.0 100.0))

(fn `EffectUpdate`
  (bind _open_width (`self.open_width`))
  (if (< 0.0 (/ (`KismetMathLibrary.FClamp` (`KismetMathLibrary.VSize` (- (`SceneComponent.K2_GetComponentLocation` (`self.rightDoor`)) (`self.K2_GetActorLocation`))) 0.0 _open_width) _open_width))
    (set `/Game/Item/Effects/BP_OpenEffect.IsStart` true (`self.openEffect`))
    (`self.K2_SetActorLocation` (`self.openEffect`) (`KismetMathLibrary.MakeVector` (.x (`self.K2_GetActorLocation` (`self.openEffect`))) (.y (`self.K2_GetActorLocation` (`self.openEffect`))) (.z (`SceneComponent.K2_GetComponentLocation` (`self.rightBox`)))) false false)))

(fn `open_the_door`
  (returns (isOpen :type Boolean))
  (bind (_open_door _isopen) (`self.Open_the_Door_width` (`SceneComponent.K2_GetComponentLocation` (`self.rightDoor`)) (`self.K2_GetActorLocation`) (* (`self.GetActorRightVector`) -1.0)))
  (if (`self.isOpen`)
    (`SceneComponent.K2_SetWorldLocation` (`self.leftDoor`) (`self.Open_the_Door_width` (`SceneComponent.K2_GetComponentLocation` (`self.leftDoor`)) (`self.K2_GetActorLocation`) (`self.GetActorRightVector`)) false false)
    (`SceneComponent.K2_SetWorldLocation` (`self.rightDoor`) _open_door false false)
    (return _isopen)))

(fn `UserConstructionScript`)