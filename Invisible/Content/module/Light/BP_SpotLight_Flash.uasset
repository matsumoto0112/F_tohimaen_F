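; Spotlight actor that flickers irregularly, like a faulty lamp.
; On BeginPlay it caches the light's intensity and rolls a small set of random frequency coefficients.
; Each Tick sums alternating cosine and sine waves of elapsed time at those frequencies, creating pseudo-random flicker without per-frame randomness.
; When the sum dips below a threshold, it dims both the spotlight and the LightBody material's Coef parameter together.
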(event `self.ReceiveBeginPlay`
  (set `self.DefaultIntencity` (`LightComponentBase.Intensity` (`self.SpotLight`)))
  (for _ (range 6)
    (`KismetArrayLibrary.Array_Add` (`self.Coefs`) (`KismetMathLibrary.RandomFloatInRange` (`self.MinCoef`) (`self.MaxCoef`)))))

(event `self.ReceiveTick`
  (params (DeltaSeconds :type "Float (single-precision)"))
  (bind _time (`self.Time`))
  (bind _tempvalue (`self.TempValue`))
  (bind _lightbody (`self.LightBody`))
  (bind _spotlight (`self.SpotLight`))
  (set `self.Time` (+ DeltaSeconds (`self.Time`)))
  (set `self.TempValue` 0.0)
  (for (_array_element _array_index) (`self.Coefs`)
    (if (`KismetMathLibrary.Conv_IntToBool` (mod _array_index 2))
      (bind _value (`self.SinX` _time _array_element))
      (set `self.TempValue` (+ _value _tempvalue))
      (else
        (bind _value_2 (`self.CosX` _time _array_element))
        (set `self.TempValue` (+ _tempvalue _value_2)))))
  (if (>= (`self.TempValue`) -1.0)
    (`LightComponent.SetIntensity` _spotlight (* (`self.DefaultIntencity`) 1.0))
    (`MeshComponent.SetScalarParameterValueOnMaterials` _lightbody "Coef" 1.0)
    (else
      (`LightComponent.SetIntensity` _spotlight (* (`self.DefaultIntencity`) 0.1))
      (`MeshComponent.SetScalarParameterValueOnMaterials` _lightbody "Coef" 0.1))))

(fn `CosX`
  (params (X :type "Float (double-precision)") (Coef :type "Float (double-precision)"))
  (returns (Value :type "Float (double-precision)"))
  (return (`KismetMathLibrary.Cos` (* X Coef))))

(fn `SinX`
  (params (X :type "Float (double-precision)") (Coef :type "Float (double-precision)"))
  (returns (Value :type "Float (double-precision)"))
  (return (`KismetMathLibrary.Sin` (* X Coef))))

(fn `UserConstructionScript`)