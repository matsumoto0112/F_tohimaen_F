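; BP_SearchManager is an enemy-side manager for a set of linked search points held in its Search array.
; SetRadius copies the manager's Radius to every point in the array.
; ViewSearch visualizes the network with short-lived green debug spheres, raised one radius along each point's up vector, and lines to the points in its Branch list.
; It has no active event logic, only these two utility functions.
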(fn `SetRadius`
  (for _array_element (`self.search`)
    (set `SearchEgde.radius` (`self.radius`) _array_element)))

(fn `UserConstructionScript`)

(fn `ViewSearch`
  (bind _returnvalue (`KismetMathLibrary.MakeColor` 0.0 1.0))
  (bind _radius (`self.radius`))
  (for _array_element (`self.search`)
    (bind _returnvalue_2 (* (`self.GetActorUpVector` _array_element) _radius))
    (bind _returnvalue_3 (+ (`self.K2_GetActorLocation` _array_element) _returnvalue_2))
    ;[1 1 1] make_draw
    (`KismetSystemLibrary.DrawDebugSphere` _returnvalue_3 _radius 12 _returnvalue 1.0 10.0)
    (for _array_element_2 (`SearchEgde.branch` _array_element)
      (`KismetSystemLibrary.DrawDebugLine` _returnvalue_3 (+ _returnvalue_2 (`self.K2_GetActorLocation` _array_element_2)) _returnvalue 1.0 10.0))))