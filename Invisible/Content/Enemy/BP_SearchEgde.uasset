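; BP_SearchEgde is an enemy-side graph node actor that links to other actors through its Branch array and can visualize those connections.
; ViewBranch draws a green debug sphere of Radius, raised by that radius along the actor's up vector, then a line and matching sphere for each Branch entry.
; The drawings last briefly, and the file holds no search or gameplay logic, as its event graph and construction script are empty.
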(event `self.ReceiveBeginPlay`)

(fn `UserConstructionScript`)

(fn `ViewBranch`
  (bind _returnvalue (`KismetMathLibrary.MakeColor` 0.0 1.0))
  (bind _radius (`self.radius`))
  (bind _returnvalue_2 (* (`self.GetActorUpVector`) _radius))
  (bind _returnvalue_3 (+ (`self.K2_GetActorLocation`) _returnvalue_2))
  ;[1 1 1] make_draw
  (`KismetSystemLibrary.DrawDebugSphere` _returnvalue_3 _radius 12 _returnvalue 1.0 10.0)
  (for _array_element (`self.branch`)
    (bind _returnvalue_4 (+ _returnvalue_2 (`self.K2_GetActorLocation` _array_element)))
    (`KismetSystemLibrary.DrawDebugLine` _returnvalue_3 _returnvalue_4 _returnvalue 1.0 10.0)
    (`KismetSystemLibrary.DrawDebugSphere` _returnvalue_4 _radius 12 _returnvalue 1.0 10.0)))