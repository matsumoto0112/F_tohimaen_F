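; BP_Enemy is an enemy Blueprint that visualises its course and vision area for debugging.
; Each Tick it draws a red sphere at itself and lines through the Courses points.
; It queries IsEyeArea, defined outside these graphs, and draws a forward vision cone, red when true and green otherwise.
; The Eyearea flag limits the detection message to the moment of entry; the capsule overlap event does nothing.
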(event `self.ReceiveTick`
  (params (DeltaSeconds :type "Float (single-precision)"))
  (`self.debugDrawCourse`)
  (bind _returnvalue (`self.IsEyeArea`))
  (`self.Debug Draw Eye Area` _returnvalue)
  (if _returnvalue
    (if (not (`self.eyearea`))
      (`KismetSystemLibrary.PrintString` "Get_Eye_Area!!"))
    (set `self.eyearea` true)
    (else
      (set `self.eyearea` false))))

(event `self.capsule.OnComponentBeginOverlap`
  (params (OverlappedComponent :type "PrimitiveComponent Object Reference") (OtherActor :type "Actor Object Reference") (OtherComp :type "PrimitiveComponent Object Reference") (OtherBodyIndex :type Integer) (bFromSweep :type Boolean) (SweepResult :type "HitResult Structure (by ref)")))

(fn `Debug Draw Eye Area`
  (params (isEyeArea :type Boolean))
  (bind _returnvalue (`self.K2_GetActorLocation`))
  (bind _returnvalue_2 (`self.GetActorForwardVector`))
  (bind _eyedeg (`self.eyeDeg`))
  (bind _eyelength (`self.eyeLength`))
  (if isEyeArea
    (`KismetSystemLibrary.DrawDebugConeInDegrees` _returnvalue _returnvalue_2 _eyelength _eyedeg _eyedeg 12 (struct :`R` 1.0 :`A` 1.0))
    (else
      (`KismetSystemLibrary.DrawDebugConeInDegrees` _returnvalue _returnvalue_2 _eyelength _eyedeg _eyedeg 12 (struct :`G` 1.0 :`A` 1.0)))))

(fn `debugDrawCourse`
  (bind _returnvalue (`self.K2_GetActorLocation`))
  (`KismetSystemLibrary.DrawDebugSphere` _returnvalue 50.0 12 (struct :`R` 1.0 :`A` 1.0))
  (if (< 0 (`KismetArrayLibrary.Array_Length` (`self.courses`)))
    (`KismetSystemLibrary.DrawDebugLine` _returnvalue (`|GetArrayItem` (`self.courses`)) (struct :`R` 1.0 :`A` 1.0))
    (for _index (range (+ (`KismetArrayLibrary.Array_Length` (`self.courses`)) 1))
      (if (< (+ _index 1) (`KismetArrayLibrary.Array_Length` (`self.courses`)))
        (`KismetSystemLibrary.DrawDebugLine` (`|GetArrayItem` (`self.courses`) _index) (`|GetArrayItem` (`self.courses`) (+ _index 1)) (struct :`R` 1.0 :`A` 1.0))))))

(fn `UserConstructionScript`)