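; Player character Blueprint with a game-over sequence that turns the view toward an enemy.
; LookAtEnemyEvent starts a per-frame looping timer that smoothly rotates control rotation toward a target, flattened to yaw.
; Once aligned, it clears the timer, waits briefly, then fades to the GameOver level.
; The capsule hit event is empty, and the enemy-cast chains that call death and look-at logic are disconnected.
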(event `self.CapsuleComponent.OnComponentHit`
  (params (HitComponent :type "PrimitiveComponent Object Reference") (OtherActor :type "Actor Object Reference") (OtherComp :type "PrimitiveComponent Object Reference") (NormalImpulse :type "Vector Structure") (Hit :type "HitResult Structure (by ref)")))

(event `LookAtEnemyEvent`
  (params (Target :type "Enemy Object Reference"))
  (`KismetSystemLibrary.K2_SetTimerDelegate` (delegate `LookAtEnemyGradually`) (`GameplayStatics.GetWorldDeltaSeconds`) true))

(event `LookAtEnemyGradually`
  (bind _returnvalue (`KismetMathLibrary.FindLookAtRotation` (`KismetMathLibrary.MakeVector` (.x (`self.K2_GetActorLocation`)) (.y (`self.K2_GetActorLocation`))) (`KismetMathLibrary.MakeVector` (.x (`self.TargetLocation`)) (.y (`self.TargetLocation`)))))
  (`Controller.SetControlRotation` (`GameplayStatics.GetPlayerController` 0) (`KismetMathLibrary.RInterpTo` (`self.K2_GetActorRotation`) _returnvalue (`GameplayStatics.GetWorldDeltaSeconds`) 3.0))
  (if (== (`self.K2_GetActorRotation`) _returnvalue :`ErrorTolerance` 1.0)
    (`KismetSystemLibrary.K2_SetTimerDelegate` (delegate `LookAtEnemyGradually`))
    (`KismetSystemLibrary.Delay` 3.0)
    (`/Game/Level/SceneChangeMacro_BP.SceneChange` "GameOver")))

(fn `UserConstructionScript`)