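; PlayerTestGameMode is a game mode Blueprint that tracks elapsed game time for the current level.
; It resets GameTime on BeginPlay and accumulates delta seconds every Tick.
; On EndPlay caused by a level transition, it writes the total to MyGameInstance_BP, replacing the stored GameTime so the value outlives the level.
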(event `self.ReceiveBeginPlay`
  (set `self.GameTime` 0.0))

(event `self.ReceiveTick`
  (params (DeltaSeconds :type "Float (single-precision)"))
  (set `self.GameTime` (+ (`self.GameTime`) DeltaSeconds)))

(event `self.ReceiveEndPlay`
  (params (EndPlayReason :type "EEndPlayReason Enum" :default "Destroyed"))
  (if (`|EnumEquality` EndPlayReason (enumliteral `EEndPlayReason` "LevelTransition"))
    (bind _asmy_game_instance_bp (cast `/Game/System/MyGameInstance_BP` (`GameplayStatics.GetGameInstance`)))
    (set `/Game/System/MyGameInstance_BP.GameTime` (`self.GameTime`) _asmy_game_instance_bp)))

(fn `UserConstructionScript`)